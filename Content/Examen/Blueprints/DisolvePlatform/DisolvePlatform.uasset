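; DisolvePlatform is a platform Blueprint that toggles a dissolve effect on its static mesh when the Disolve Material input is pressed.
; A FlipFlop alternates between playing a timeline forward and reversing it from the end, with the timeline driving the DisolutionValue material parameter.
; The reverse branch also sets AllowBurn to one, which is never reset here.
; Dynamic material instance setup exists but is disconnected.
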(event `InputAction|Disolve Material`
  (params (Key :type "Key Structure"))
  (:`Pressed`
    (`/Engine/EditorBlueprintResources/StandardMacros.FlipFlop`
      (:`A`
        (bind (_direction _newtrack_2) (`Timeline|Timeline_0` :!label _label)
          (:`Update`
            (`MeshComponent.SetScalarParameterValueOnMaterials` (`self.StaticMesh`) "DisolutionValue" _newtrack_2))))
      (:`B`
        (`MeshComponent.SetScalarParameterValueOnMaterials` (`self.StaticMesh`) "AllowBurn" 1.0)
        (goto _label :!via `ReverseFromEnd`)))))

(fn `UserConstructionScript`)